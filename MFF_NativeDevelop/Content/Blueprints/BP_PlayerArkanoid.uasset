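; Player paddle Blueprint for an Arkanoid game, moved along the world X axis through Enhanced Input.
; BeginPlay adds the Arkanoid mapping context to the first player's input subsystem.
; IA_Move passes its action value to AddMovementInput as the scale.
; An earlier solution using PaddleSpeed and actor world offsets remains disconnected, along with a debug print.
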(event `self.ReceiveBeginPlay`
  (`EnhancedInputSubsystemInterface.AddMappingContext` (pcsubsystem `EnhancedInputLocalPlayerSubsystem` (`GameplayStatics.GetPlayerController` 0)) "/Game/Input/IMC_Arkanoid.IMC_Arkanoid" 0 (struct)))

(event `EnhancedInput|/Game/Input/IA_Move`
  (params (ActionValue :type "Float (double-precision)") (ElapsedSeconds :type "Float (double-precision)") (TriggeredSeconds :type "Float (double-precision)") (InputAction :type "InputAction Object Reference" :default "/Game/Input/IA_Move.IA_Move"))
  ;[1 1 1] First solution
)

(event `EnhancedInput|/Game/Input/IA_Move`
  (params (ActionValue :type "Float (double-precision)") (ElapsedSeconds :type "Float (double-precision)") (TriggeredSeconds :type "Float (double-precision)") (InputAction :type "InputAction Object Reference" :default "/Game/Input/IA_Move.IA_Move"))
  ;[1 1 1] Lecture
  (:`Triggered`
    (`self.AddMovementInput` (1.0 0.0 0.0) ActionValue)))

(fn `UserConstructionScript`)